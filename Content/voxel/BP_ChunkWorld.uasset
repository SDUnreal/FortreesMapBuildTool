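; BP_ChunkWorld is a voxel-folder Blueprint that appears to be a test for steering and drawing a target vertex.
; X, Y and Z movement axes accumulate positive input into their TargetVertex component, zeroing the other two.
; BeginPlay starts a looping one-second timer, presumably bound to DrawVertexEvent, which calls DrawVertex and prints TargetVertex.
; Overlap, Tick and the construction script are empty.
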(event `InputAxis|XMovement`
  (params (AxisValue :type "Float (single-precision)"))
  (bind (_targetvertex_x _targetvertex_y _targetvertex_z) (`KismetMathLibrary.BreakVector` (`self.TargetVertex`)))
  ;[1 1 1] Input Action
  (if (> AxisValue 0.0)
    (set `self.TargetVertex` (`KismetMathLibrary.MakeVector` (+ AxisValue _targetvertex_x)))))

(event `InputAxis|YMovement`
  (params (AxisValue :type "Float (single-precision)"))
  (bind (_targetvertex_x _targetvertex_y _targetvertex_z) (`KismetMathLibrary.BreakVector` (`self.TargetVertex`)))
  ;[1 1 1] Input Action
  (if (> AxisValue 0.0)
    (set `self.TargetVertex` (`KismetMathLibrary.MakeVector` 0.0 (+ AxisValue _targetvertex_y)))))

(event `InputAxis|ZMovement`
  (params (AxisValue :type "Float (single-precision)"))
  (bind (_targetvertex_x _targetvertex_y _targetvertex_z) (`KismetMathLibrary.BreakVector` (`self.TargetVertex`)))
  ;[1 1 1] Input Action
  (if (> AxisValue 0.0)
    (set `self.TargetVertex` (`KismetMathLibrary.MakeVector` 0.0 0.0 (+ AxisValue _targetvertex_z)))))

(event `self.ReceiveBeginPlay`
  (`KismetSystemLibrary.K2_SetTimerDelegate` (`|CreateDelegate` :!event `Draw Vertex Event`) 1.0 true))

(fn `Draw Vertex Event`
  (`self.DrawVertex` 1.0)
  (`KismetSystemLibrary.PrintString` (`KismetStringLibrary.Conv_VectorToString` (`self.TargetVertex`))))

(fn `UserConstructionScript`)